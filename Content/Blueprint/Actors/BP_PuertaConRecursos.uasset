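; BP_PuertaConRecursos is a resource-gate actor that collects a required quantity of one item from the player.
; BeginPlay copies the required Quantity into CurrentQuantity as the remaining amount.
; On collision with BP_ThirdPersonCharacter, it removes as much of that item as is held or still needed from BPInventory, allowing partial deliveries.
; When the remainder reaches zero it only prints a completion message, with no door-opening logic.
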(event EventOnCollide
  (params (ColActor :type Actor%20Object%20Reference))
  (bind _asbp_third_person_character (Utilities|Casting|CastToBP_ThirdPersonCharacter ColActor))
  (if (.ReturnValue (Utilities|Map|Find (Variables|/Game/Blueprint/Components/BP_Inventory.BP_Inventory_C|GetInventory (Variables|/Game/ThirdPerson/Blueprints/BP_ThirdPersonCharacter.BP_ThirdPersonCharacter_C|GetBP_Inventory _asbp_third_person_character)) (.rowname (Variables|Default|GetItem))))
    (Default|RemovefromInventory (Variables|/Game/ThirdPerson/Blueprints/BP_ThirdPersonCharacter.BP_ThirdPersonCharacter_C|GetBP_Inventory _asbp_third_person_character) (.rowname (Variables|Default|GetItem)) (Math|Integer|Min(Integer) (.Value (Utilities|Map|Find (Variables|/Game/Blueprint/Components/BP_Inventory.BP_Inventory_C|GetInventory (Variables|/Game/ThirdPerson/Blueprints/BP_ThirdPersonCharacter.BP_ThirdPersonCharacter_C|GetBP_Inventory _asbp_third_person_character)) (.rowname (Variables|Default|GetItem)))) (Variables|Default|GetCurrentQuantity)))
    (bind _output_get (Variables|Default|SetCurrentQuantity (- (Variables|Default|GetCurrentQuantity) (Math|Integer|Min(Integer) (.Value (Utilities|Map|Find (Variables|/Game/Blueprint/Components/BP_Inventory.BP_Inventory_C|GetInventory (Variables|/Game/ThirdPerson/Blueprints/BP_ThirdPersonCharacter.BP_ThirdPersonCharacter_C|GetBP_Inventory _asbp_third_person_character)) (.rowname (Variables|Default|GetItem)))) (Variables|Default|GetCurrentQuantity)))))
    (if (<= _output_get 0)
      (Development|PrintText "complete pedido"))))

(event EventBeginPlay
  (Variables|Default|SetCurrentQuantity (Variables|Default|GetQuantity)))

(fn ConstructionScript)