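; BP_Inventory is a component that tracks item quantities in a map keyed by item name.
; AddItemToInventory adds the given quantity to an existing entry or creates a new one.
; RemoveFromInventory subtracts a quantity from an existing entry and deletes the entry when the result drops to zero or below, ignoring items that are absent.
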(fn AddItemtoInventory
  (params (ItemName :type Name) (ItemQuantity :type Integer))
  (bind _inventory (Variables|Default|GetInventory))
  (bind (_value _returnvalue) (Utilities|Map|Find _inventory ItemName))
  (if _returnvalue
    (Utilities|Map|Add (Variables|Default|GetInventory) ItemName (+ _value ItemQuantity))
    (else
      (Utilities|Map|Add (Variables|Default|GetInventory) ItemName ItemQuantity))))

(fn RemovefromInventory
  (params (ItemToRemove :type Name) (Quantity :type Integer))
  (bind _inventory (Variables|Default|GetInventory))
  (bind _inventory_2 (Variables|Default|GetInventory))
  (bind (_value _returnvalue) (Utilities|Map|Find _inventory ItemToRemove))
  (bind _returnvalue_2 (- _value Quantity))
  (if _returnvalue
    (if (> _returnvalue_2 0)
      (Utilities|Map|Add _inventory_2 ItemToRemove _returnvalue_2)
      (else
        (Utilities|Map|Remove _inventory_2 ItemToRemove)))))